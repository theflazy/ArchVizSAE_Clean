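; BP_windowsTurn is an interactable double window that the player opens and closes with the E key.
; Box overlap with the FPV character enables or disables input and shows or hides the Widget1 component.
; E flips IsWindowsClosed and plays or reverses a timeline that lerps both panes' relative yaw in opposite directions.
; A separate macro, not called here, adds a viewport widget with mouse cursor and Game-and-UI input.
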(event OnComponentBeginOverlap(Box)
  (params (OverlappedComponent :type Primitive%20Component%20Object%20Reference) (OtherActor :type Actor%20Object%20Reference) (OtherComp :type Primitive%20Component%20Object%20Reference) (OtherBodyIndex :type Integer) (bFromSweep :type Boolean) (SweepResult :type Hit%20Result%20Structure%20%28by%20ref%29))
  ;[1 1 1] Enable/diable input
  (Utilities|Casting|CastToFPV OtherActor)
  (Input|EnableInput (Game|GetPlayerController 0))
  (Rendering|SetVisibility (Variables|Default|GetWidget1) true false))

(event OnComponentEndOverlap(Box)
  (params (OverlappedComponent :type Primitive%20Component%20Object%20Reference) (OtherActor :type Actor%20Object%20Reference) (OtherComp :type Primitive%20Component%20Object%20Reference) (OtherBodyIndex :type Integer))
  ;[1 1 1] Enable/diable input
  (Utilities|Casting|CastToFPV OtherActor)
  (Input|DisableInput (Game|GetPlayerController 0))
  (Rendering|SetVisibility (Variables|Default|GetWidget1) false false))

(event EventBeginPlay
  ;[1 1 1] Get Player ref
  (bind _asfpv (Utilities|Casting|CastToFPV (Game|GetPlayerCharacter 0)))
  (Variables|Default|SetPlayer%20Ref _asfpv)
  (Rendering|SetVisibility (Variables|Default|GetWidget1) false false))

(event Input|KeyboardEvents|E
  (params (Key :type Key%20Structure))
  (:Pressed
    (if (Variables|Default|GetIsWindowsClosed)
      (Variables|Default|SetIsWindowsClosed false)
      (bind _alpha (Timeline|Timeline_0 Play)
        (:Update
          (Utilities|FlowControl|Sequence
            (:then_0
              (Transformation|SetRelativeRotation (Variables|Default|GetwindowLeft) (Math|Rotator|MakeRotator 0.0 0.0 (Math|Float|Lerp 0.0 (Math|Float|SelectFloat 0.0 -9e+01 false) _alpha)) false false))
            (:then_1
              (Transformation|SetRelativeRotation (Variables|Default|GetwindowRight) (Math|Rotator|MakeRotator 0.0 0.0 (Math|Float|Lerp 0.0 (Math|Float|SelectFloat 0.0 9e+01 false) _alpha)) false false)))))
      (else
        (Variables|Default|SetIsWindowsClosed true)
        (Timeline|Timeline_0 Reverse)))))

(fn ConstructionScript)