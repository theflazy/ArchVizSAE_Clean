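; BP_Door1WayPush is an interactable door that swings one way when the player left-clicks within range.
; A box overlap with the FPV character enables input and shows a widget, and leaving disables input and hides it.
; Each click toggles the closed flag and plays or reverses a timeline, which lerps the door's relative yaw between zero and a fixed negative angle.
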(event OnComponentBeginOverlap(Box)
  (params (OverlappedComponent :type Primitive%20Component%20Object%20Reference) (OtherActor :type Actor%20Object%20Reference) (OtherComp :type Primitive%20Component%20Object%20Reference) (OtherBodyIndex :type Integer) (bFromSweep :type Boolean) (SweepResult :type Hit%20Result%20Structure%20%28by%20ref%29))
  ;[1 1 1] Enable/diable input
  (Utilities|Casting|CastToFPV OtherActor)
  (Input|EnableInput (Game|GetPlayerController 0))
  (Rendering|SetVisibility (Variables|Default|GetWidget1) true false))

(event OnComponentEndOverlap(Box)
  (params (OverlappedComponent :type Primitive%20Component%20Object%20Reference) (OtherActor :type Actor%20Object%20Reference) (OtherComp :type Primitive%20Component%20Object%20Reference) (OtherBodyIndex :type Integer))
  ;[1 1 1] Enable/diable input
  (Utilities|Casting|CastToFPV OtherActor)
  (Input|DisableInput (Game|GetPlayerController 0))
  (Rendering|SetVisibility (Variables|Default|GetWidget1) false false))

(event EventBeginPlay
  ;[1 1 1] Get Player ref
  (bind _asfpv (Utilities|Casting|CastToFPV (Game|GetPlayerCharacter 0)))
  (Variables|Default|SetPlayerRef _asfpv)
  (Rendering|SetVisibility (Variables|Default|GetWidget1) false false))

(event Input|MouseEvents|LeftMouseButton
  (params (Key :type Key%20Structure :default "None"))
  (:Pressed
    (if (Variables|Default|GetIsDoorClosed)
      (Variables|Default|SetIsDoorClosed false)
      (bind _alpha (Timeline|DoorInteract_TL Play)
        (:Update
          (Transformation|SetRelativeRotation (Variables|Default|GetDoor) (Math|Rotator|MakeRotator 0.0 0.0 (Math|Float|Lerp 0.0 (Math|Float|SelectFloat 0.0 -9e+01 false) _alpha)) false false)))
      (else
        (Variables|Default|SetIsDoorClosed true)
        (Timeline|DoorInteract_TL Reverse)))))

(fn ConstructionScript)