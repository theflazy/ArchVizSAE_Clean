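; BP_WindowsSlidingAuto is an automatic two-panel sliding window that opens when the FPV actor enters its trigger Box and closes when it leaves.
; Both overlap events wait half a second, then play or reverse a vector Timeline.
; The Timeline value sets WindowRight's relative location, while WindowLeft uses the X-negated value plus a small offset.
; A float Timeline with Lerp-based positions is left in the graph but never runs.
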(event OnComponentBeginOverlap(Box)
  (params (OverlappedComponent :type Primitive%20Component%20Object%20Reference) (OtherActor :type Actor%20Object%20Reference) (OtherComp :type Primitive%20Component%20Object%20Reference) (OtherBodyIndex :type Integer) (bFromSweep :type Boolean) (SweepResult :type Hit%20Result%20Structure%20%28by%20ref%29))
  (Utilities|Casting|CastToFPV OtherActor)
  (Utilities|FlowControl|Delay 0.5)
  ;[1 1 1] Timeline as vector
  (bind _door_sliding (Timeline|Timeline_0 Play)
    (:Update
      (Utilities|FlowControl|Sequence
        (:then_0
          (Transformation|SetRelativeLocation (Variables|Default|GetWindow%20right) _door_sliding false false))
        (:then_1
          (Transformation|SetRelativeLocation (Variables|Default|Getwindow%20left) (+ (* _door_sliding "-1.000000,0.000000, 0") "-4.187733, 0, 0") false false))))))

(event OnComponentEndOverlap(Box)
  (params (OverlappedComponent :type Primitive%20Component%20Object%20Reference) (OtherActor :type Actor%20Object%20Reference) (OtherComp :type Primitive%20Component%20Object%20Reference) (OtherBodyIndex :type Integer))
  (Utilities|Casting|CastToFPV OtherActor)
  (Utilities|FlowControl|Delay 0.5)
  ;[1 1 1] Timeline as vector
  (bind _door_sliding (Timeline|Timeline_0 Reverse)
    (:Update
      (Utilities|FlowControl|Sequence
        (:then_0
          (Transformation|SetRelativeLocation (Variables|Default|GetWindow%20right) _door_sliding false false))
        (:then_1
          (Transformation|SetRelativeLocation (Variables|Default|Getwindow%20left) (+ (* _door_sliding "-1.000000,0.000000, 0") "-4.187733, 0, 0") false false))))))

(fn ConstructionScript)