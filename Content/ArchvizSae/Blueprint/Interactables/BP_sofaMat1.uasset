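; Interactable archviz sofa that lets the player swap its mesh material through a UI widget.
; Entering the overlap area calls the FPV character's event for this sofa's Object1–5 slot and creates the widget.
; Tick shows or removes the widget, cursor and prompt according to the player's Use flag.
; While overlapping, Tick also polls the character's per-sofa button flags to apply one of three materials.
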(event OnComponentBeginOverlap(OverlapArea)
  (params (OverlappedComponent :type Primitive%20Component%20Object%20Reference) (OtherActor :type Actor%20Object%20Reference) (OtherComp :type Primitive%20Component%20Object%20Reference) (OtherBodyIndex :type Integer) (bFromSweep :type Boolean) (SweepResult :type Hit%20Result%20Structure%20%28by%20ref%29))
  (bind _playercharref (Variables|Default|GetPlayerCharref))
  (Variables|Default|SetbIsOverlap true)
  ;[1 1 1] Choose Object
  (if (Variables|Default|GetbObject1?)
    (Default|Object1 _playercharref)
    ;[1 1 1] Create Widget
    (bind _returnvalue (UserInterface|CreateWidget (Variables|Default|GetWidget) (Game|GetPlayerController 0) :!label _label))
    (elif (Variables|Default|GetbObject2?)
      (Default|Object2 _playercharref)
      (goto _label)
      (elif (Variables|Default|GetbObject3?)
        (Default|Object3 _playercharref)
        (goto _label)
        (elif (Variables|Default|GetbObject4?)
          (Default|Object4 _playercharref)
          (goto _label)
          (elif (Variables|Default|GetbObject5?)
            (Default|Object5 _playercharref)
            (goto _label)))))))

(event OnComponentEndOverlap(OverlapArea)
  (params (OverlappedComponent :type Primitive%20Component%20Object%20Reference) (OtherActor :type Actor%20Object%20Reference) (OtherComp :type Primitive%20Component%20Object%20Reference) (OtherBodyIndex :type Integer))
  (bind _returnvalue (Game|GetPlayerController 0))
  (Variables|Default|SetbIsOverlap false)
  ;[1 1 1] Create Widget On Overlap
  (Widget|RemovefromParent (stale OnComponentBeginOverlap(OverlapArea) _returnvalue))
  (Input|SetInputModeGameOnly _returnvalue)
  (Variables|/Script/Engine.PlayerController|SetbShowMouseCursor _returnvalue false)
  (Development|SetHiddeninGame (Variables|Default|GetWidget1) true false)
  (Variables|/Game/ArchvizSae/Blueprint/FPV.FPV_C|SetbUse (Variables|Default|GetPlayerCharref) false))

(event EventBeginPlay
  ;[1 1 1] Begin Play & Cast
  (bind _asfpv (Utilities|Casting|CastToFPV (Game|GetPlayerCharacter 0)))
  (Variables|Default|SetPlayerCharref _asfpv))

(event EventTick
  (params (DeltaSeconds :type Float%20%28single-precision%29))
  (bind _returnvalue (Game|GetPlayerController 0))
  (bind _returnvalue_2 (Game|GetPlayerController 0))
  (bind _playercharref (Variables|Default|GetPlayerCharref))
  ;[1 1 1] Change Mat With widget
  (Utilities|FlowControl|Sequence
    (:then_0
      ;[1 1 1] Create Widget
      (if (Variables|Default|GetbIsOverlap)
        (if (Variables|/Game/ArchvizSae/Blueprint/FPV.FPV_C|GetbUse (Variables|Default|GetPlayerCharref))
          (Utilities|FlowControl|DoOnce false :!label _label
            (:Completed
              (UserInterface|Viewport|AddtoViewport (stale OnComponentBeginOverlap(OverlapArea) _returnvalue) 0)
              (Variables|/Script/Engine.PlayerController|SetbShowMouseCursor _returnvalue_2 true)
              (Input|SetInputModeGameandUI _returnvalue_2 0 "DoNotLock" true)
              (Development|SetHiddeninGame (Variables|Default|GetWidget1) true false)))
          (elif (Variables|Default|GetbIsOverlap)
            (Widget|RemovefromParent (stale OnComponentBeginOverlap(OverlapArea) _returnvalue))
            (Variables|/Script/Engine.PlayerController|SetbShowMouseCursor _returnvalue false)
            (Input|SetInputModeGameOnly _returnvalue)
            (Development|SetHiddeninGame (Variables|Default|GetWidget1) false false)
            (goto _label Reset)))))
    (:then_1
      (if (Variables|Default|GetbIsOverlap)
        (if (Variables|/Game/ArchvizSae/Blueprint/FPV.FPV_C|GetbObject1? _playercharref)
          (|CollapseGraph_0 :!label _label_2)
          (elif (Variables|/Game/ArchvizSae/Blueprint/FPV.FPV_C|GetbObject2? _playercharref)
            (goto _label_2 execute2)
            (elif (Variables|/Game/ArchvizSae/Blueprint/FPV.FPV_C|GetbObject3? _playercharref)
              (goto _label_2 execute3)
              (elif (Variables|/Game/ArchvizSae/Blueprint/FPV.FPV_C|GetbObject4? _playercharref)
                (goto _label_2 execute4)
                (elif (Variables|/Game/ArchvizSae/Blueprint/FPV.FPV_C|GetbObject5? _playercharref)
                  (goto _label_2 execute5))))))))))

(fn ConstructionScript)