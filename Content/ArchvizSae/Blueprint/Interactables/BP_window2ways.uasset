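; Interactable two-way window that the FPV player opens and closes with E while inside its trigger box, which also shows a prompt widget.
; A dot product between the player direction and the Scene forward vector picks the swing side.
; A timeline lerps Door yaw up to 90 degrees either way and reverses to close.
; Tick prints that dot product on screen for debugging.
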(event OnComponentBeginOverlap(Box)
  (params (OverlappedComponent :type Primitive%20Component%20Object%20Reference) (OtherActor :type Actor%20Object%20Reference) (OtherComp :type Primitive%20Component%20Object%20Reference) (OtherBodyIndex :type Integer) (bFromSweep :type Boolean) (SweepResult :type Hit%20Result%20Structure%20%28by%20ref%29))
  ;[1 1 1] Enable/diable input
  (Utilities|Casting|CastToFPV OtherActor)
  (Input|EnableInput (Game|GetPlayerController 0))
  (Rendering|SetVisibility (Variables|Default|GetWidget1) true false))

(event OnComponentEndOverlap(Box)
  (params (OverlappedComponent :type Primitive%20Component%20Object%20Reference) (OtherActor :type Actor%20Object%20Reference) (OtherComp :type Primitive%20Component%20Object%20Reference) (OtherBodyIndex :type Integer))
  ;[1 1 1] Enable/diable input
  (Utilities|Casting|CastToFPV OtherActor)
  (Input|DisableInput (Game|GetPlayerController 0))
  (Rendering|SetVisibility (Variables|Default|GetWidget1) false false))

(event EventTick
  (params (DeltaSeconds :type Float%20%28single-precision%29))
  (bind _scene (Variables|Default|GetScene))
  (Development|PrintString (Utilities|String|ToString(Float) (Math|Vector|DotProduct (Math|Vector|Normalize (- (Transformation|GetWorldLocation _scene) (Transformation|GetActorLocation (Variables|Default|GetPlayerRef)))) (Math|Vector|GetForwardVector _scene))) true true "(R=0.000000,G=0.660000,B=1.000000,A=1.000000)" DeltaSeconds))

(event EventBeginPlay
  ;[1 1 1] Get Player ref
  (bind _asfpv (Utilities|Casting|CastToFPV (Game|GetPlayerCharacter 0)))
  (Variables|Default|SetPlayerRef _asfpv)
  (Rendering|SetVisibility (Variables|Default|GetWidget1) false false))

(event Input|KeyboardEvents|E
  (params (Key :type Key%20Structure))
  (bind _scene (Variables|Default|GetScene))
  (:Pressed
    (if (Variables|Default|GetIsDoorClosed)
      (Variables|Default|SetIsDoorClosed false)
      (Variables|Default|SetdotProduct (Math|Vector|DotProduct (Math|Vector|Normalize (- (Transformation|GetWorldLocation _scene) (Transformation|GetActorLocation (Variables|Default|GetPlayerRef)))) (Math|Vector|GetForwardVector _scene)))
      (bind (_direction _alpha) (Timeline|Timeline_0 Play)
        (:Update
          (Transformation|SetRelativeRotation (Variables|Default|GetDoor) (Math|Rotator|MakeRotator 0.0 0.0 (Math|Float|Lerp 0.0 (Math|Float|SelectFloat 9e+01 -9e+01 (>= (Variables|Default|GetdotProduct) 0.0)) _alpha)) false false))
        (:Finished
          (switch Utilities|FlowControl|Switch|SwitchonETimelineDirection _direction
            (:Backward
              (Variables|Default|SetIsDoorClosed true)))))
      (else
        (Timeline|Timeline_0 Reverse)))))

(fn ConstructionScript)