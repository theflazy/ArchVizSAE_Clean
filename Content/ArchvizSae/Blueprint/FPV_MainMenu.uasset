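; FPV_MainMenu is a first-person Blueprint that brings up the main menu of the ArchvizSae project.
; On BeginPlay it opens the menu media source on the MainMenuVideo player and shows the mouse cursor.
; It then creates the video widget and adds it to the viewport, followed by the menu widget.
; The construction script snaps FPGun to the GripPoint socket on Mesh2P.
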(event EventBeginPlay
  (Media|MediaPlayer|OpenSource (Variables|Default|GetMain%20Menu%20Video) "/Game/ArchvizSae/Materials/MainMenu/MainMenu_MediaSource.MainMenu_MediaSource")
  (Variables|/Script/Engine.PlayerController|SetbShowMouseCursor (Game|GetPlayerController 0) true)
  (bind _returnvalue (UserInterface|CreateWidget "/Game/ArchvizSae/Blueprint/Widget/HUD_MainMenu/BP_Video_MainMenu.BP_Video_MainMenu_C"))
  (UserInterface|Viewport|AddtoViewport _returnvalue 0)
  (bind _returnvalue_2 (UserInterface|CreateWidget "/Game/ArchvizSae/Blueprint/Widget/HUD_MainMenu/BP_MainMenu.BP_MainMenu_C"))
  (UserInterface|Viewport|AddtoViewport _returnvalue_2 0))

(fn ConstructionScript
  (Transformation|AttachComponentToComponent (Variables|Default|GetFP_Gun) (Variables|MyCharacter|GetMesh2P) "GripPoint" "SnapToTarget" "SnapToTarget" "SnapToTarget" true))